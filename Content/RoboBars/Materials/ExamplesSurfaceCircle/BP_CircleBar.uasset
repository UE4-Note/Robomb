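; BP_CircleBar is an example actor for a circular progress bar material, pairing a mesh with a percentage title.
; The construction script creates a dynamic material instance from the Material variable on the mesh's first element.
; Each tick sets that instance's Progress parameter to a fixed value, while the title shows a 0–100% sine oscillation driven by game time and Speed, so the two are not linked.
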(event EventBeginPlay)

(event Collision|EventActorBeginOverlap
  (params (OtherActor :type Actor%20Object%20Reference)))

(event EventTick
  (params (DeltaSeconds :type Float%20%28single-precision%29))
  ;[1 1 1] Update progress bar
  (Rendering|Material|SetScalarParameterValue (Variables|Default|GetMaterialInstance) "Progress" 0.2 :!class /Script/Engine.MaterialInstanceDynamic)
  (Rendering|Components|TextRender|SetText (Variables|Default|GetTitle) (Utilities|Text|ToText(String) (Utilities|String|BuildString(Integer) "" "" (Math|Float|Round (* (* (+ (Math|Trig|Sin(Radians) (* (Utilities|Time|GetTimeSeconds) (Variables|Default|GetSpeed))) 1.0) 0.5) 1e+02)) "%"))))

(fn ConstructionScript
  (bind _returnvalue (Rendering|Material|CreateDynamicMaterialInstance (Variables|Default|GetMesh) 0 (Variables|Default|GetMaterial) "None" :!class /Script/Engine.PrimitiveComponent))
  (Variables|Default|SetMaterialInstance _returnvalue))